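; BP_HealthStats stores a maximum and current value for HP and MP.
; Set HP and MP overwrites all four values directly, with no clamping.
; Get Stats for HUD returns them as truncated integer text, along with HP and MP progress bar fractions normalized from zero to each maximum.
; The event graph is inactive, so the Blueprint does nothing until one of these functions is called.
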(event EventBeginPlay)

(event EventTick
  (params (DeltaSeconds :type Float%20%28single-precision%29)))

(fn GetStatsforHUD
  (return (Utilities|Text|ToText(Integer) (Math|Float|Truncate (Variables|Default|GetMax_HP))) (Utilities|Text|ToText(Integer) (Math|Float|Truncate (Variables|Default|GetCurrent_HP))) (Utilities|Text|ToText(Integer) (Math|Float|Truncate (Variables|Default|GetMax_MP))) (Utilities|Text|ToText(Integer) (Math|Float|Truncate (Variables|Default|GetCurrent_MP))) (Math|Float|NormalizetoRange (Variables|Default|GetCurrent_HP) 0.0 (Variables|Default|GetMax_HP)) (Math|Float|NormalizetoRange (Variables|Default|GetCurrent_MP) 0.0 (Variables|Default|GetMax_MP))))

(fn SetHPandMP
  (params (Set_Max_HP :type Float%20%28single-precision%29) (Set_Current_HP :type Float%20%28single-precision%29) (Set_Max_MP :type Float%20%28single-precision%29) (Set_Current_MP :type Float%20%28single-precision%29))
  (Variables|Default|SetMax_HP Set_Max_HP)
  (Variables|Default|SetCurrent_HP Set_Current_HP)
  (Variables|Default|SetMax_MP Set_Max_MP)
  (Variables|Default|SetCurrent_MP Set_Current_MP))